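; Base pickup actor that can be thrown and heals a B_Golem_Test_2 it hits.
; Throw turns on physics and launches the root along the Arrow's forward vector, with impulse strength interpolated from the Force input.
; A hit while moving either applies HealthAdded as negative damage to the golem and destroys the pickup, or stops physics on anything else.
; ChangePickupCollision sets the root's response to a given collision channel.
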(event OnComponentHit(Root)
  (params (HitComponent :type Primitive%20Component%20Object%20Reference) (OtherActor :type Actor%20Object%20Reference) (OtherComp :type Primitive%20Component%20Object%20Reference) (NormalImpulse :type Vector :default "0, 0, 0") (Hit :type Hit%20Result%20Structure%20%28by%20ref%29))
  (if (Variables|Default|GetIsMoving)
    (if (== (Utilities|GetClass OtherActor) "/Game/Test_Blueprints/B_Golem_Test_2.B_Golem_Test_2_C")
      (Game|Damage|ApplyDamage OtherActor (- 0.0 (Variables|Default|GetHealthAdded)) 0 self)
      (Actor|DestroyActor)
      (else
        (Physics|SetSimulatePhysics (Variables|Default|GetRoot) false)))))

(event EventBeginPlay)

(event EventThrow
  (params (Force :type Float%20%28single-precision%29))
  (Physics|SetSimulatePhysics (Variables|Default|GetRoot) true)
  (Physics|AddImpulse (Variables|Default|GetRoot) (* (Math|Vector|GetForwardVector (Variables|Default|GetArrow)) (Math|Float|Lerp 1.5e+02 1.2e+03 Force)) "None" true)
  (Variables|Default|SetIsMoving true))

(event EventChangePickupCollision
  (params (Channel :type ECollisionChannel%20Enum :default "ECC_WorldStatic") (Response :type ECollisionResponse%20Enum :default "ECR_Ignore"))
  (Collision|SetCollisionResponsetoChannel (Variables|Default|GetRoot) Channel Response))

(fn ConstructionScript)