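; Player character Blueprint with camera-yaw movement, a charged jump, and pickup and charged throwing of objects.
; Timelines charge jump height and throw force while input is held, scaling a ring and an arrow indicator through dynamic materials.
; A forward box trace finds objects to attach to a hand socket, with messages driving them and the AnimInstance.
; It also decrements health on damage and flags a brief jump-recovery window after walking into a fall.
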(event Custom|ThrowObject
  (Utilities|IsValid (Variables|Default|GetHeldObject)
    (:Is%20Valid
      (Default|BeginThrow (Variables|Default|GetAnim))
      (Transformation|DetachFromActor (Variables|Default|GetHeldObject) "KeepWorld" "KeepWorld" "KeepWorld")
      (Class|IPickup|Throw(Message) (Variables|Default|GetHeldObject) (Variables|Default|GetThrowForce))
      (Variables|Default|SetHeldObject 0))))

(event Game|Damage|EventAnyDamage
  (params (Damage :type Float%20%28single-precision%29) (DamageType :type Damage%20Type%20Object%20Reference) (InstigatedBy :type Controller%20Object%20Reference) (DamageCauser :type Actor%20Object%20Reference))
  (Variables|Default|SetcurrentHealth (- (Variables|Default|GetcurrentHealth) 1.0)))

(event EventBeginPlay
  (bind _animref (Class|ICharacter|SetPlayerRef(Message) (Components|SkeletalMesh|GetAnimInstance (Variables|Character|GetMesh)) self))
  (Variables|Default|SetAnim _animref)
  (bind _returnvalue (Rendering|Material|CreateDynamicMaterialInstance (Variables|Default|GetArrow_plane) 0 "/Game/Blueprints_Jamie/Material/M_Arrow.M_Arrow" "None" :!class /Script/Engine.PrimitiveComponent))
  (Variables|Material|SetArrow_Mat _returnvalue)
  (bind _returnvalue_2 (Rendering|Material|CreateDynamicMaterialInstance (Variables|Default|GetJumpRing) 0 "/Game/Blueprints_Jamie/Material/MI_JumpRing.MI_JumpRing" "None" :!class /Script/Engine.PrimitiveComponent))
  (Variables|Material|SetJumpRing_Mat _returnvalue_2))

(event EventOnMovementModeChanged
  (params (PrevMovementMode :type EMovementMode%20Enum :default "MOVE_None") (NewMovementMode :type EMovementMode%20Enum :default "MOVE_None") (PrevCustomMode :type Byte :default 0) (NewCustomMode :type Byte :default 0))
  (if (and (Utilities|Enum|Equal(Enum) PrevMovementMode "MOVE_Walking") (Utilities|Enum|Equal(Enum) NewMovementMode "MOVE_Falling"))
    (Variables|Default|SetCanRecoverJump true)
    (Utilities|FlowControl|Delay 2.0)
    (Variables|Default|SetCanRecoverJump false)))

(event Input|ActionEvents|InputActionJump
  (params (Key :type Key%20Structure))
  (:Pressed
    (Rendering|SetVisibility (Variables|Default|GetJumpRing) true false)
    (bind _jumpcharge (Timeline|JumpCharge PlayFromStart)
      (:Update
        (Variables|Default|SetJumpCharge_val _jumpcharge)
        (Rendering|Material|SetScalarParameterValue (Variables|Material|GetJumpRing_Mat) "Percent" _jumpcharge :!class /Script/Engine.MaterialInstanceDynamic)
        (Transformation|SetRelativeScale3D (Variables|Default|GetJumpRing) (Math|Vector|Lerp(Vector) "1.000000,1.000000,0.000000" "5.000000,5.000000,5.000000" _jumpcharge)))))
  (:Released
    (Utilities|FlowControl|Sequence
      (:then_0
        (Timeline|JumpCharge Stop))
      (:then_1
        (Variables|/Script/Engine.CharacterMovementComponent|SetJumpZVelocity (Variables|Character|GetCharacterMovement) (Math|Float|Lerp 3e+02 9e+02 (Variables|Default|GetJumpCharge_val)))
        (Character|Jump)
        (Rendering|SetVisibility (Variables|Default|GetJumpRing) false false)))))

(event Input|ActionEvents|InputActionPickup
  (params (Key :type Key%20Structure))
  (bind (_start _end _orientation) (CallFunction|GetPickupTraceVectors))
  (:Pressed
    (Utilities|IsValid (Variables|Default|GetHeldObject)
      (:Is%20Not%20Valid
        (bind _outhit (Class|KismetSystemLibrary|BoxTraceSingleforObjects _start _end "25.000000,1.000000,50.000000" _orientation (Utilities|Array|MakeArray "ObjectTypeQuery7") false 0 "Persistent" true "(R=1.000000,G=0.000000,B=0.000000,A=1.000000)" "(R=0.000000,G=1.000000,B=0.000000,A=1.000000)" 2.0))
        (if (.bBlockingHit (Collision|BreakHitResult _outhit))
          (Variables|Default|SetHeldObject (.HitActor (Collision|BreakHitResult _outhit)))
          (Class|IPickup|ChangePickupCollision(Message) (.HitActor (Collision|BreakHitResult _outhit)) "ECC_Pawn" "ECR_Ignore")
          (Transformation|AttachComponentToComponent (.HitActor (Collision|BreakHitResult _outhit)) (Variables|Character|GetMesh) "Pickup_Socket" "SnapToTarget" "SnapToTarget" "KeepWorld" false)
          (Default|BeginPickup (Variables|Default|GetAnim))
          (Variables|Default|SetCanThrow true))))))

(event Input|ActionEvents|InputActionThrow
  (params (Key :type Key%20Structure))
  (:Pressed
    (if (Variables|Default|GetCanThrow)
      (Rendering|SetVisibility (Variables|Default|GetArrow_plane) true false)
      (bind _alpha (Timeline|ArrowIndicator PlayFromStart)
        (:Update
          (Variables|Default|SetThrowForce _alpha)
          (Rendering|Material|SetScalarParameterValue (Variables|Material|GetArrow_Mat) "Percent" _alpha :!class /Script/Engine.MaterialInstanceDynamic)
          (Transformation|SetRelativeScale3D (Variables|Default|GetScene) (Math|Vector|MakeVector 1.5 (Math|Float|Lerp 0.5 6.0 _alpha) 1.5))))))
  (:Released
    (Utilities|FlowControl|Sequence
      (:then_0
        (Timeline|ArrowIndicator Stop))
      (:then_1
        (Rendering|SetVisibility (Variables|Default|GetArrow_plane) false false)
        (Variables|Default|SetCanThrow false)
        (CallFunction|ThrowObject)))))

(event Input|AxisEvents|InputAxisRight
  (params (AxisValue :type Float%20%28single-precision%29))
  (Variables|Default|SetRight AxisValue)
  (if (> (Math|Float|Absolute(Float) AxisValue) 0.0)
    (Pawn|Input|AddMovementInput (Math|Vector|GetForwardVector (Math|Rotator|MakeRotator 0.0 0.0 (.yaw (Pawn|GetControlRotation :!class /Script/Engine.Pawn)))) AxisValue false)))

(event Input|AxisEvents|InputAxisForward
  (params (AxisValue :type Float%20%28single-precision%29))
  (Variables|Default|SetForwards AxisValue)
  (if (> (Math|Float|Absolute(Float) AxisValue) 0.0)
    (Pawn|Input|AddMovementInput (Math|Vector|GetRightVector (Math|Rotator|MakeRotator 0.0 0.0 (.yaw (Pawn|GetControlRotation :!class /Script/Engine.Pawn)))) (* AxisValue -1.0) false)))

(event Input|KeyboardEvents|K
  (params (Key :type Key%20Structure))
  (:Pressed
    (Default|HideBone (Variables|Default|GetAnim))))

(fn ConstructionScript
  (Transformation|AttachComponentToComponent (Variables|Default|GetArrow1) (Variables|Character|GetMesh) "Forward" "SnapToTarget" "KeepRelative" "KeepRelative" true)
  (Transformation|AttachComponentToComponent (Variables|Default|GetScene) (Variables|Character|GetMesh) "root" "KeepRelative" "KeepRelative" "KeepRelative" true))

(fn GetPickupTraceVectors
  (bind _arrow1 (Variables|Default|GetArrow1))
  (bind _returnvalue (Math|Vector|GetForwardVector _arrow1))
  (bind _returnvalue_2 (Transformation|GetWorldLocation _arrow1))
  (bind (_x _y) (Math|Vector|BreakVector _returnvalue))
  (bind _returnvalue_3 (Math|Vector|MakeVector _x _y 0.0))
  (bind _returnvalue_4 (* _returnvalue_3 5.0))
  (bind _returnvalue_5 (+ _returnvalue_2 _returnvalue_4))
  (return _returnvalue_5 (+ _returnvalue_5 (* _returnvalue_3 5e+01)) (Math|Rotator|MakeRotator 0.0 0.0 (.Yaw (Math|Rotator|BreakRotator (Math|Rotator|CombineRotators (Transformation|GetWorldRotation (Variables|Default|GetArrow1)) "0,90.000000, 0"))))))

(fn GetPlayerAxis
  (return (Input|AxisValues|GetForward) (Input|AxisValues|GetRight)))

(fn SetPlayerRef
  (params (Player :type BP%20Player%20Char%20Object%20Reference))
  (return 0))