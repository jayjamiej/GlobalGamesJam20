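; BP_Camera is a shared camera actor that keeps both the Character and the Golem in view.
; Each Character movement update moves it to the midpoint between the Character and the Golem's CameraOffset component.
; The spring arm length scales with the distance between those two points, clamped to a minimum, so the view zooms out as they separate.
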(event Custom|MoveCam
  (params (DeltaSeconds :type Float%20%28single-precision%29) (OldLocation :type Vector) (OldVelocity :type Vector))
  (Variables|Default|SetOffset (- (Transformation|GetActorLocation (Variables|Default|GetCharacter)) (Transformation|GetWorldLocation (Variables|/Game/Test_Blueprints/B_Golem_Test_2.B_Golem_Test_2_C|GetCameraOffset (Variables|Default|GetGolem)))))
  (Transformation|SetActorLocation (+ (Transformation|GetWorldLocation (Variables|/Game/Test_Blueprints/B_Golem_Test_2.B_Golem_Test_2_C|GetCameraOffset (Variables|Default|GetGolem))) (/ (Variables|Default|GetOffset) 2.0)) false false)
  (Variables|/Script/Engine.SpringArmComponent|SetTargetArmLength (Variables|Default|GetSpringArm) (Math|Float|Clamp(Float) (* (Math|Vector|VectorLength (Variables|Default|GetOffset)) 1.25) 5e+02 1e+06)))

(event EventBeginPlay
  (Character|BindEventtoOnCharacterMovementUpdated (Variables|Default|GetCharacter) (delegate Custom|MoveCam)))

(fn ConstructionScript)